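; BP_Floor is an actor that builds a square tiled floor, with all its logic in the construction script.
; Nested loops over plus and minus half of Size add a FloorTile static mesh component at fixed spacing per grid cell.
; Each tile gets its own dynamic instance of Material.
; The actor's world location is added to each tile's relative location, so tiles are centered on the actor only at the world origin.
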(fn `UserConstructionScript`
  (bind (_returnvalue_x _returnvalue_y _returnvalue_z) (`KismetMathLibrary.BreakVector` (`self.K2_GetActorLocation` self)))
  (bind _returnvalue (/ (`self.Size`) 2))
  (bind _returnvalue_2 (/ (`self.Size`) 2))
  (for _index (range (* _returnvalue_2 -1) (+ _returnvalue_2 1))
    (for _index_2 (range (* _returnvalue -1) (+ _returnvalue 1))
      (bind _returnvalue_3 (`AddComponent|NODE_AddStaticMeshComponent-1`))
      (`StaticMeshComponent.SetStaticMesh` _returnvalue_3 (`self.Floor Tile`))
      (`SceneComponent.K2_SetRelativeLocation` _returnvalue_3 (`KismetMathLibrary.MakeVector` (+ (* _index_2 100) _returnvalue_x) (+ _returnvalue_y (* _index 100)) _returnvalue_z) false false)
      (`PrimitiveComponent.CreateDynamicMaterialInstance` _returnvalue_3 0 (`self.Material`) "None"))))